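; Interactable mill actor that toggles the rotation of its SMHouseVar02Extra component each time it is interacted with.
; Interact checks IsSpinning and calls either RotateMill or StopMill, which update that flag.
; RotateMill plays a half-speed timeline that lerps the component's relative pitch through a full turn, and StopMill halts the timeline in place.
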(event `/Game/Base/Blueprints/Interfaces/BPI_Interaction.Interact`
  (if (not (`self.isSpinning?`))
    (`self.Rotate Mill`)
    (else
      (`self.Stop Mill`))))

(event `Rotate Mill`
  (`TimelineComponent.SetPlayRate` (`self.Timeline - Mill Animation`) 0.5)
  (set `self.isSpinning?` true)
  (bind (_direction _alpha) (`Timeline|Timeline - Mill Animation` :!label _label)
    (:`Update`
      (`SceneComponent.K2_SetRelativeRotation` (`self.SM_House_Var02_Extra`) (`KismetMathLibrary.MakeRotator` 0.0 (`KismetMathLibrary.Lerp` 0.0 360.0 _alpha)) false false))))

(event `Stop Mill`
  (set `self.isSpinning?` false)
  (goto _label :!via `Stop`))

(fn `UserConstructionScript`
  (`parent.UserConstructionScript`))