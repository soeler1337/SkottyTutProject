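; PC_GamePlay is the gameplay player controller that owns the on-screen HUD.
; On BeginPlay it creates a WB_HUD widget, stores it as WidgetHUD and adds it to the viewport.
; Its UpdateWheels event forwards an amount to the HUD widget, acting as the entry point for wheel display updates.
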(event `self.ReceiveBeginPlay`
  (`parent.ReceiveBeginPlay`)
  (`self.Create HUD`))

(event `Create HUD`
  (bind _returnvalue (`|CreateWidget` "/Game/Base/Widgets/WB_HUD.WB_HUD_C" self))
  (bind _output_get (set `self.Widget_HUD` _returnvalue))
  (`UserWidget.AddToViewport` _output_get 0))

(event `/Game/Base/Blueprints/Interfaces/BPI_PlayerController.UpdateWheels`
  (params (amount :type Integer))
  (`/Game/Base/Widgets/WB_HUD.Update Wheels` (`self.Widget_HUD`) amount))

(fn `UserConstructionScript`
  (`parent.UserConstructionScript`))