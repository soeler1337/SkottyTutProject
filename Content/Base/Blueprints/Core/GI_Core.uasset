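; GI_Core is the core Game Instance that owns the game's save file.
; On Init it loads the SG_SaveFile from its slot, or creates and immediately saves a new one if none exists.
; A debug flag can delete the existing save first.
; It exposes GetSaveFile for access to the cached object and a SaveGame event to write it back to disk.
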(event `self.ReceiveInit`
  ;[1 0 0] Debug Only - Save Löschen
  (if (`self.delete Save file`)
    (`GameplayStatics.DeleteGameInSlot` (`self.Save File Name`)))
  (bind _returnvalue (`GameplayStatics.DoesSaveGameExist` (`self.Save File Name`)))
  (if _returnvalue
    (bind _returnvalue_2 (`GameplayStatics.LoadGameFromSlot` (`self.Save File Name`)))
    (bind _assg_save_file (cast `/Game/Base/Blueprints/Core/SG_SaveFile` _returnvalue_2))
    (set `self.SaveFile` _assg_save_file)
    (else
      (bind _returnvalue_3 (`GameplayStatics.CreateSaveGameObject` "/Game/Base/Blueprints/Core/SG_SaveFile.SG_SaveFile_C"))
      (bind _output_get (set `self.SaveFile` _returnvalue_3))
      (`GameplayStatics.SaveGameToSlot` _output_get (`self.Save File Name`)))))

(event `/Game/Base/Blueprints/Interfaces/BPI_GameInstance.saveGame`
  (`GameplayStatics.SaveGameToSlot` (`self.SaveFile`) (`self.Save File Name`)))

(fn `getSaveFile`
  (returns (saveFile :type "/Game/Base/Blueprints/Core/SG_SaveFile Object Reference"))
  (return (`self.SaveFile`)))