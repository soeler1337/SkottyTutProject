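; Inventory component that keeps the player's Wheels count and persists it in the save file.
; On BeginPlay it reads the saved count from the game instance and feeds it through AddWheels, so loading also triggers a save.
; AddWheels adds the amount, sends the new total to player controller 0, then writes it to the save file and saves immediately through the game instance.
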(event `self.ReceiveBeginPlay`
  (bind _savefile (message `/Game/Base/Blueprints/Interfaces/BPI_GameInstance.getSaveFile` (`GameplayStatics.GetGameInstance`)))
  (`self.addWheels` (`/Game/Base/Blueprints/Core/SG_SaveFile.wheels` _savefile)))

(fn `addWheels`
  (params (amount :type Integer))
  (bind _output_get (set `self.wheels` (+ amount (`self.wheels`))))
  (message `/Game/Base/Blueprints/Interfaces/BPI_PlayerController.UpdateWheels` (`GameplayStatics.GetPlayerController` 0) _output_get)
  (bind _savefile (message `/Game/Base/Blueprints/Interfaces/BPI_GameInstance.getSaveFile` (`GameplayStatics.GetGameInstance`)))
  (set `/Game/Base/Blueprints/Core/SG_SaveFile.wheels` (`self.wheels`) _savefile)
  (message `/Game/Base/Blueprints/Interfaces/BPI_GameInstance.saveGame` (`GameplayStatics.GetGameInstance`)))