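; Player character with Enhanced Input look, yaw-relative movement, sprint, interaction and wheel pickup.
; Every tick a Visibility line trace sends a focus message to the hit actor and stores it as the current interactable, clearing it on a miss.
; The interact input messages that stored actor, and CollectWheel adds wheels to the inventory component before destroying the wheel actor.
; Sprint switches max walk speed while held.
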(event `self.ReceiveTick`
  (params (DeltaSeconds :type "Float (single-precision)"))
  (`self.interactTrace`))

(event `/Game/Base/Blueprints/Interfaces/BPI_Interaction.collectWheel`
  (params (amount :type Integer) (`Wheel Actor` :type "Actor Object Reference"))
  (`/Game/Base/Blueprints/Components/C_Inventory.addWheels` (`self.C_Inventory`) amount)
  (`self.K2_DestroyActor` `Wheel Actor`))

(event `EnhancedInput|/Game/Base/Inputs/IA_Look`
  (params (ActionValue :type "Vector2D Structure") (ElapsedSeconds :type "Float (double-precision)") (TriggeredSeconds :type "Float (double-precision)") (InputAction :type "InputAction Object Reference" :default "/Game/Base/Inputs/IA_Look.IA_Look"))
  (bind _mousesensity (`self.MouseSensity`))
  ;[0.7332 1 0.7717] CameraMovement
  (:`Triggered`
    (`self.AddControllerYawInput` (* ActionValue_X _mousesensity))
    (`self.AddControllerPitchInput` (* (* ActionValue_Y _mousesensity) -1.0))))

(event `EnhancedInput|/Game/Base/Inputs/IA_Move`
  (params (ActionValue :type "Vector2D Structure") (ElapsedSeconds :type "Float (double-precision)") (TriggeredSeconds :type "Float (double-precision)") (InputAction :type "InputAction Object Reference" :default "/Game/Base/Inputs/IA_Move.IA_Move"))
  (bind (_returnvalue_roll _returnvalue_pitch _returnvalue_yaw) (`KismetMathLibrary.BreakRotator` (`self.GetControlRotation`)))
  ;[0.2118 0.9002 1] Movenment
  (:`Triggered`
    (`self.AddMovementInput` (`KismetMathLibrary.GetForwardVector` (`KismetMathLibrary.MakeRotator` 0.0 0.0 _returnvalue_yaw)) ActionValue_Y)
    (`self.AddMovementInput` (`KismetMathLibrary.GetRightVector` (`KismetMathLibrary.MakeRotator` 0.0 0.0 _returnvalue_yaw)) ActionValue_X)))

(event `EnhancedInput|/Game/Base/Inputs/IA_Sprint`
  (params (ActionValue :type Boolean) (ElapsedSeconds :type "Float (double-precision)") (TriggeredSeconds :type "Float (double-precision)") (InputAction :type "InputAction Object Reference" :default "/Game/Base/Inputs/IA_Sprint.IA_Sprint"))
  ;[1 1 1] Sprint
  (:`Started`
    (set `CharacterMovementComponent.MaxWalkSpeed` 600.0 (`self.CharacterMovement`)))
  (:`Canceled`
    (set `CharacterMovementComponent.MaxWalkSpeed` 200.0 (`self.CharacterMovement`) :!label _label))
  (:`Completed`
    (goto _label)))

(event `EnhancedInput|/Game/Base/Inputs/IA_Interact`
  (params (ActionValue :type Boolean) (ElapsedSeconds :type "Float (double-precision)") (TriggeredSeconds :type "Float (double-precision)") (InputAction :type "InputAction Object Reference" :default "/Game/Base/Inputs/IA_Interact.IA_Interact"))
  ;[1 1 1] Interaction
  (:`Started`
    (bind _current_interactable (`self.Current Interactable`)
      (:`then`
        (message `/Game/Base/Blueprints/Interfaces/BPI_Interaction.Interact` _current_interactable))
      (:`else`))))

(fn `interactTrace`
  (locals (traceDistance :type "Float (single-precision)" :default 400.0))
  (bind _camera (`self.Camera`))
  (bind _returnvalue (`SceneComponent.K2_GetComponentLocation` _camera))
  (bind (_outhit _returnvalue_2) (`KismetSystemLibrary.LineTraceSingle` (+ _returnvalue (* (`SceneComponent.GetForwardVector` _camera) (`SpringArmComponent.TargetArmLength` (`self.SpringArm`)))) (+ _returnvalue (* (`SceneComponent.GetForwardVector` _camera) (`local.traceDistance`))) "TraceTypeQuery1"))
  (if _returnvalue_2
    (bind (_bblockinghit _binitialoverlap _time _distance _location _impactpoint _normal _impactnormal _physmat _hitactor) (`GameplayStatics.BreakHitResult` _outhit))
    (message `/Game/Base/Blueprints/Interfaces/BPI_Interaction.Focus` _hitactor)
    (set `self.Current Interactable` _hitactor)
    (else
      (set `self.Current Interactable` null))))

(fn `UserConstructionScript`)